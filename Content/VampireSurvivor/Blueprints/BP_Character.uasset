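; BP_Character is a Vampire Survivor-style character that automatically targets and damages nearby enemies.
; Each Tick without a valid target, FindNearestEnemies gathers every BP_Enemy within AgroRadius, and one is picked at random rather than by proximity.
; With a valid target, Tick applies fixed damage every frame and calls FiredEvent.
; The timer it resets each frame targets an empty event, so it does not throttle attacks.
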(event `Fired_Event`)

(event `self.ReceiveTick`
  (params (DeltaSeconds :type "Float (single-precision)"))
  (if (`KismetSystemLibrary.IsValid` (`self.CurrentEnemy`))
    (`KismetSystemLibrary.K2_SetTimerDelegate` (delegate `Fired_Event`) 1.2)
    (`/Game/VampireSurvivor/Blueprints/Enemies/BP_Enemy.DoDamage` (`self.CurrentEnemy`) 34.0)
    (`self.Fired_Event`)
    (else
      (`self.FindNearestEnemies`)
      (if (> (`KismetArrayLibrary.Array_Length` (`self.NearbyEnemies`)) 0)
        (set `self.CurrentEnemy` (`KismetArrayLibrary.Array_Random` (`self.NearbyEnemies`)))
        (`self.Fired_Event`)))))

(fn `FindNearestEnemies`
  (`|ExecutionSequence`
    (:`then_0`
      (`KismetArrayLibrary.Array_Clear` (`self.NearbyEnemies`)))
    (:`then_1`
      (bind _outactors (`GameplayStatics.GetAllActorsOfClass` "/Game/VampireSurvivor/Blueprints/Enemies/BP_Enemy.BP_Enemy_C"))
      (for _array_element _outactors
        (if (<= (`self.GetDistanceTo` _array_element) (`self.AgroRadius`))
          (`KismetArrayLibrary.Array_Add` (`self.NearbyEnemies`) _array_element))))))

(fn `UserConstructionScript`)